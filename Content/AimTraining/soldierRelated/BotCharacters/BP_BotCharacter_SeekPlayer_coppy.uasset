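; Bot character variant for aim training that seeks out the nearest living enemy player as its target.
; It extends the parent's FindClosestTarget event with an extra player search while the bot is alive.
; When no valid target exists, it scans the Squad game state's PlayerArray, skipping teammates and admin cameras, and sets the closest living controlled pawn as CurrentTarget.
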(event `self.Find Closest Target`
  (`parent.Find Closest Target`)
  (if (not (`self.Dead`))
    (`self.Find Enemy in Player States`)))

(fn `Find Enemy in Player States`
  (locals (Closest :type "Float (double-precision)" :default 99999.0) (`Closest Enemy` :type "Actor Object Reference"))
  (`self.Current Target`
    (:`then`)
    (:`else`
      (for _array_element (`GameStateBase.PlayerArray` (`/Game/Gameplay/BP_GameplayFunctionLibrary.GetSquadGameState`))
        (bind _assqplayer_controller (cast `SQPlayerController` (`self.GetOwner` _array_element)))
        (bind _returnvalue (`Controller.K2_GetPawn` _assqplayer_controller))
        (if (and (!= (`SQPlayerController.GetTeam` _assqplayer_controller) (`SQTeamInterface.GetTeamId`)) (not (`SQPlayerController.IsAdminCamera` _assqplayer_controller)) (`KismetSystemLibrary.IsValid` _returnvalue))
          (bind _returnvalue_2 (`self.GetDistanceTo` _returnvalue self))
          (if (and (`self.Is Actor Alive` _returnvalue) (< _returnvalue_2 (`local.Closest`)))
            (set `local.Closest` _returnvalue_2)
            (set `local.Closest Enemy` _returnvalue))))
      (bind _closest_enemy (`local.Closest Enemy`)
        (:`then`
          (`self.Set Current Target` _closest_enemy))
        (:`else`)))))

(fn `UserConstructionScript`
  (`parent.UserConstructionScript`))