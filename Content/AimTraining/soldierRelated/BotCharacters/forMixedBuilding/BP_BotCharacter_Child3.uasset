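; Child bot character Blueprint for aim training that adds render-based tick throttling to its parent bot.
; BeginPlay runs the parent logic, enables tick and starts a looping one-second timer.
; The timer keeps actor tick enabled only if the bot was rendered within the last second, saving work for unseen bots.
; Tick and construction script simply call the parent implementations.
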(event `self.ReceiveBeginPlay`
  (`parent.ReceiveBeginPlay`)
  (`self.SetActorTickEnabled` true)
  (`KismetSystemLibrary.K2_SetTimerDelegate` (delegate `timer that controls tick`) 1.0 true))

(event `timer that controls tick`
  (if (`self.WasRecentlyRendered` 1.0)
    (`self.SetActorTickEnabled` true)
    (else
      (`self.SetActorTickEnabled` false))))

(event `self.ReceiveTick`
  (params (DeltaSeconds :type "Float (single-precision)"))
  (`parent.ReceiveTick` DeltaSeconds))

(fn `UserConstructionScript`
  (`parent.UserConstructionScript`))