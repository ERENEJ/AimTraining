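; BP_BotCharacter_Child2_Concentrate is an aim-training bot character variant that saves performance by pausing ticking while off screen.
; On BeginPlay it adds a PawnSensing component and starts a looping one-second timer.
; The timer uses WasRecentlyRendered to toggle tick on the actor, character movement, noise emitter and added sensing component.
; An unwired fragment, marked TODO, would destroy the AI controller's PawnSensing if sensing stays costly.
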(event `self.ReceiveBeginPlay`
  (`parent.ReceiveBeginPlay`)
  (`self.SetActorTickEnabled` true)
  (`KismetSystemLibrary.K2_SetTimerDelegate` (delegate `CustomEvent`) 1.0 true)
  (bind _returnvalue (`AddComponent|NODE_AddPawnSensingComponent-0`)))

(event `CustomEvent`
  (if (`self.WasRecentlyRendered` 1.0)
    (`self.SetActorTickEnabled` true)
    (`ActorComponent.SetComponentTickEnabled` (`self.CharacterMovement`) true)
    (`ActorComponent.SetComponentTickEnabled` (`self.PawnNoiseEmitter`) true)
    (`ActorComponent.SetComponentTickEnabled` (stale `self.ReceiveBeginPlay` _returnvalue) true)
    (else
      (`self.SetActorTickEnabled` false)
      (`ActorComponent.SetComponentTickEnabled` (`self.CharacterMovement`) false)
      (`ActorComponent.SetComponentTickEnabled` (`self.PawnNoiseEmitter`) false)
      (`ActorComponent.SetComponentTickEnabled` (stale `self.ReceiveBeginPlay` _returnvalue) false))))

(event `self.ReceiveTick`
  (params (DeltaSeconds :type "Float (single-precision)"))
  (`parent.ReceiveTick` DeltaSeconds))

(fn `UserConstructionScript`
  (`parent.UserConstructionScript`))