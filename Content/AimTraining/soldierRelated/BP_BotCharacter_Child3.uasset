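; Child bot soldier for aim training that patrols back and forth between its spawn point and the location of its Sphere component.
; A looping timer flip-flops AI MoveTo between the two points.
; Another timer revives the bot when health drops to 1 or below, then crouches and uncrouches it to restore the standing pose.
; A one-second render check toggles actor, movement, noise emitter and runtime-added pawn sensing ticks to save performance.
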(event `self.ReceiveBeginPlay`
  (`parent.ReceiveBeginPlay`)
  (`self.SetActorTickEnabled` true)
  (`KismetSystemLibrary.K2_SetTimerDelegate` (delegate `timer that controls tick`) 1.0 true)
  (bind _returnvalue (`AddComponent|NODE_AddPawnSensingComponent-0`))
  (`KismetSystemLibrary.K2_SetTimerDelegate` (delegate `CustomEvent_0`) 3.0 true)
  (`KismetSystemLibrary.K2_SetTimerDelegate` (delegate `RandomWonder`) (`self.LoopTime`) true)
  (set `self.EndPosition` (`SceneComponent.K2_GetComponentLocation` (`self.Sphere`)))
  (set `self.firstPosition` (`self.K2_GetActorLocation`))
  (`|AIMoveTo` self (`self.EndPosition`) null))

(event `timer that controls tick`
  (if (`self.WasRecentlyRendered` 1.0)
    (`self.SetActorTickEnabled` true)
    (`ActorComponent.SetComponentTickEnabled` (`self.CharacterMovement`) true)
    (`ActorComponent.SetComponentTickEnabled` (`self.PawnNoiseEmitter`) true)
    (`ActorComponent.SetComponentTickEnabled` (stale `self.ReceiveBeginPlay` _returnvalue) true)
    (else
      (`self.SetActorTickEnabled` false)
      (`ActorComponent.SetComponentTickEnabled` (`self.CharacterMovement`) false)
      (`ActorComponent.SetComponentTickEnabled` (`self.PawnNoiseEmitter`) false)
      (`ActorComponent.SetComponentTickEnabled` (stale `self.ReceiveBeginPlay` _returnvalue) false))))

(event `RandomWonder`
  (`/Engine/EditorBlueprintResources/StandardMacros.FlipFlop`
    (:`A`
      (`|AIMoveTo` self (`self.firstPosition`) null))
    (:`B`
      (`|AIMoveTo` self (`self.EndPosition`) null))))

(event `self.ReceiveTick`
  (params (DeltaSeconds :type "Float (single-precision)"))
  (`parent.ReceiveTick` DeltaSeconds))

(event `CustomEvent_0`
  (if (<= (`/Game/Blueprints/AI/AutomatedWeapons/HealthComponent.Health` (`self.HealthComponent`)) 1.0)
    (`self.Server Revive`)
    ;[1 1 1] When soldier revives this functions needed for standing position
    (`self.Crouch`)
    (`self.UnCrouch`)))

(fn `UserConstructionScript`
  (`parent.UserConstructionScript`))