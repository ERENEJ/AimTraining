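; Pop-up soldier target variant for aim training that periodically teleports to a new spot, extending its parent's BeginPlay and Tick.
; A looping timer moves it to a random reachable navigation point around its current location, resetting its rotation.
; It only jumps when recently rendered; otherwise the timer event disables its actor tick until it is seen again.
; Unconnected leftovers include timer pausing and a move-to attempt noted as not working.
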(event `self.ReceiveBeginPlay`
  (`parent.ReceiveBeginPlay`)
  (`KismetSystemLibrary.K2_SetTimerDelegate` (delegate `PopUpTeleport`) 7.0 true))

(event `PopUpTeleport`
  (if (`self.WasRecentlyRendered` 1.0)
    (`self.SetActorTickEnabled` true)
    (`self.K2_TeleportTo` (`NavigationSystemV1.K2_GetRandomReachablePointInRadius` (`self.K2_GetActorLocation`) 2500.0 null null))
    (else
      (`self.SetActorTickEnabled` false))))

(event `self.ReceiveTick`
  (params (DeltaSeconds :type "Float (single-precision)"))
  (`parent.ReceiveTick` DeltaSeconds))

(fn `UserConstructionScript`
  (`parent.UserConstructionScript`))