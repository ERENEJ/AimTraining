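; Usable reset actor for the killhouse challenge in aim training, which randomly repopulates bot targets when used.
; Prompt events add or remove it as a SQHUD line-of-sight actor, with hiding also closing radial menus, though ShouldDisplayPrompt always returns false.
; On use it beeps, waits briefly, then server-revives each BP_BotCharacter_Child2 on a coin flip.
; The notice widget and its delayed fade-out sit inside that bot loop.
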(event `self.BPDisplayPrompt`
  (params (User :type "Controller Object Reference"))
  (cast `SQPlayerState` (`Controller.PlayerState` User))
  (bind _asplayer_controller (cast `PlayerController` User))
  (bind _assqhud (cast `SQHUD` (`PlayerController.GetHUD` _asplayer_controller)))
  (`SQHUD.AddLineOfSightActor` _assqhud self))

(event `self.BPHidePrompt`
  (bind _return_value (`/Game/Gameplay/BP_GameplayFunctionLibrary.GetSquadPlayerController` 0))
  (`/Engine/EditorBlueprintResources/StandardMacros.IsValid` _return_value
    (:`Is Valid`
      (bind _assqhud (cast `SQHUD` (`PlayerController.GetHUD` _return_value)))
      (bind _foundwidgets (`WidgetBlueprintLibrary.GetAllWidgetsOfClass` "/Game/UI/RadialMenu/WidgetBaseTypes/BaseRadialMenu.BaseRadialMenu_C"))
      (for _array_element _foundwidgets
        (`/Game/UI/RadialMenu/WidgetBaseTypes/BaseRadialMenu.CloseSelf` _array_element))
      (`SQHUD.RemoveLineOfSightActor` _assqhud self))))

(event `self.BPOnUsed`
  (params (User :type "Controller Object Reference"))
  (`GameplayStatics.PlaySound2D` "/aimTraining/AimTraining/VanillaRefsForCook/Start_Beep.Start_Beep" 1.0 0.5 0.0 null null)
  (`KismetSystemLibrary.Delay` 0.5)
  (bind _outactors (`GameplayStatics.GetAllActorsOfClass` "/aimTraining/AimTraining/soldierRelated/BotCharacters/child2ForCustomCQB/BP_BotCharacter_Child2.BP_BotCharacter_Child2_C"))
  (for _array_element _outactors
    (if (`KismetMathLibrary.RandomBool`)
      (`/Game/Blueprints/AI/AI_Soldier/BP_BotCharacter.Server Revive` _array_element)
      (bind _returnvalue (`|CreateWidget` "/aimTraining/AimTraining/VanillaRefsForCook/W_VolumeWidget_KillhouseChallengeReset.W_VolumeWidget_KillhouseChallengeReset_C" (`GameplayStatics.GetPlayerController` 0) 3.0))
      (`UserWidget.AddToViewport` _returnvalue 0)
      (`KismetSystemLibrary.Delay` 3.0)
      (`/Game/Blueprints/Tutorial/TutorialVolumeWidgets/W_VolumeWidget.Fade Out` _returnvalue))))

(fn `GetInterfaceTeam`
  (returns (ReturnValue :type Integer))
  (return (`self.Team`)))

(fn `GetUsableData`
  (returns (ReturnValue :type "SQUsableData Structure"))
  (return (`self.Usable Data`)))

(fn `ShouldDisplayPrompt`
  (params (User :type "Controller Object Reference"))
  (returns (ReturnValue :type Boolean))
  (return false))

(fn `UserConstructionScript`)