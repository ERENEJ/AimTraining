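; Flick-aim training target that jumps to a new spot whenever it takes damage.
; BeginPlay records its position, and each hit teleports it to a random reachable navigation point nearby, with one of two coin-flip X/Z offsets and zeroed rotation.
; Each landing becomes the next search origin, so the target can wander from its start.
; Height-correction nodes and the parent BeginPlay call are left unconnected.
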(event `self.ReceiveBeginPlay`
  (set `self.positionOfTarget` (`self.K2_GetActorLocation`)))

(event `self.ReceiveActorBeginOverlap`
  (params (OtherActor :type "Actor Object Reference"))
  (`parent.ReceiveActorBeginOverlap` OtherActor))

(event `self.ReceiveTick`
  (params (DeltaSeconds :type "Float (single-precision)"))
  (`parent.ReceiveTick` DeltaSeconds))

(event `self.ReceiveAnyDamage`
  (params (Damage :type "Float (single-precision)") (DamageType :type "DamageType Object Reference") (InstigatedBy :type "Controller Object Reference") (DamageCauser :type "Actor Object Reference"))
  (if (`KismetMathLibrary.RandomBool`)
    (`self.K2_TeleportTo` (+ (`NavigationSystemV1.K2_GetRandomReachablePointInRadius` (`self.positionOfTarget`) 250.0 null null) (`KismetMathLibrary.MakeVector` (`KismetMathLibrary.RandomFloatInRange` 30.0 40.0) 0.0 -20.0)))
    (bind _output_get (set `self.positionOfTarget` (`self.K2_GetActorLocation`)))
    (else
      (`self.K2_TeleportTo` (+ (`NavigationSystemV1.K2_GetRandomReachablePointInRadius` (`self.positionOfTarget`) 250.0 null null) (`KismetMathLibrary.MakeVector` (`KismetMathLibrary.RandomFloatInRange` -30.0 -45.0) 0.0 20.0)))
      (bind _output_get_2 (set `self.positionOfTarget` (`self.K2_GetActorLocation`))))))

(fn `UserConstructionScript`)